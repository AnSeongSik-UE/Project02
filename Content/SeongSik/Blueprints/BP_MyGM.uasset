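; Game mode Blueprint that processes character interactions with actors, currently picking up and sitting.
; S2A_Interact forwards to ProcessInteract, which checks the target's CanInteract and branches on the requested action.
; Pickup snaps the actor to the character's mesh socket; Sit aligns the character using seat and body sockets, attaches it and stops movement.
; Successful attachment records the interaction on the character, locks the target and adjusts its collision.
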(event `S2A_Interact`
  (params (InCharacter :type "/Game/SeongSik/Blueprints/Character/BP_MyCharacter Object Reference") (InActor :type "/Game/SeongSik/Blueprints/Objects/BP_InteractableActor Object Reference") (WantAct :type "/Game/SeongSik/Blueprints/Character/EN_Interactons Enum" :default "NewEnumerator0"))
  (`self.ProcessInteract` InCharacter InActor WantAct))

(fn `ProcessInteract`
  (params (InCharacter :type "/Game/SeongSik/Blueprints/Character/BP_MyCharacter Object Reference") (InActor :type "/Game/SeongSik/Blueprints/Objects/BP_InteractableActor Object Reference") (WantAct :type "/Game/SeongSik/Blueprints/Character/EN_Interactons Enum" :default "NewEnumerator0"))
  (bind _inactor (`local.InActor`))
  (bind _inactor_2 (`local.InActor`))
  (bind (_returnvalue_location _returnvalue_rotation) (`KismetMathLibrary.BreakTransform` (`SceneComponent.GetSocketTransform` (`InteractableActor.StaticMesh` (`local.InActor`)) "mesh_sit" "RTS_World")))
  (bind _returnvalue_location_2 (`KismetMathLibrary.BreakTransform` (`SceneComponent.GetSocketTransform` (`Character.Mesh` (`local.InCharacter`)) "sitting_location" "RTS_Actor")))
  ; 상호작용 가능 여부 검증
  (`/Game/SeongSik/Blueprints/Objects/BP_InteractableActor.CanInteract` (`local.InActor`)
    (:`then`
      (switch `/Game/SeongSik/Blueprints/Character/EN_Interactons` (`local.WantAct`)
        (:`NewEnumerator2`
          ; 들기
          (bind _returnvalue (`self.K2_AttachToComponent` (`local.InActor`) (`Character.Mesh` (`local.InCharacter`)) "pickup_location" "SnapToTarget" "KeepWorld" "KeepWorld" true))
          (if _returnvalue
            (set `/Game/SeongSik/Blueprints/Character/BP_MyCharacter.InteractedActor` _inactor_2 (`local.InCharacter`))
            (set `/Game/SeongSik/Blueprints/Objects/BP_InteractableActor.CanInteract` false _inactor_2)
            (`PrimitiveComponent.SetCollisionEnabled` (`InteractableActor.StaticMesh` _inactor_2) "NoCollision")
            (set `/Game/SeongSik/Blueprints/Character/BP_MyCharacter.Interaction` (`local.WantAct`) (`local.InCharacter`))))
        (:`NewEnumerator1`
          ; 앉을 위치, 방향 계산
          (`self.K2_SetActorLocationAndRotation` (`local.InCharacter`) (- _returnvalue_location _returnvalue_location_2) _returnvalue_rotation false false)
          ; 앉기
          (bind _returnvalue_2 (`self.K2_AttachToComponent` (`local.InCharacter`) (`InteractableActor.StaticMesh` (`local.InActor`)) "None" "KeepWorld" "KeepWorld" "KeepWorld" true))
          (if _returnvalue_2
            (set `/Game/SeongSik/Blueprints/Character/BP_MyCharacter.InteractedActor` _inactor (`local.InCharacter`))
            (set `/Game/SeongSik/Blueprints/Objects/BP_InteractableActor.CanInteract` false _inactor)
            (`PrimitiveComponent.SetCollisionEnabled` (`InteractableActor.StaticMesh` _inactor) "QueryOnly")
            (set `/Game/SeongSik/Blueprints/Character/BP_MyCharacter.Interaction` (`local.WantAct`) (`local.InCharacter`))
            (`CharacterMovementComponent.SetMovementMode` (`Character.CharacterMovement` (`local.InCharacter`)) "MOVE_None" 0)))))
    (:`else`)))

(fn `UserConstructionScript`)