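; BP_Platform is a platform that hands ownership requests and actor attachment to the game mode.
; Characters entering or leaving its ControlArea trigger a C2S event, which asks BP_MyGM to process platform ownership.
; Interactable actors overlapping its StaticMesh trigger a second C2S event, which asks BP_MyGM to attach them to the platform.
; Tick and construction only call the parent implementation.
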(event `self.ReceiveTick`
  (params (DeltaSeconds :type "Float (single-precision)"))
  (`parent.ReceiveTick` DeltaSeconds))

(event `self.ControlArea.OnComponentBeginOverlap`
  (params (OverlappedComponent :type "PrimitiveComponent Object Reference") (OtherActor :type "Actor Object Reference") (OtherComp :type "PrimitiveComponent Object Reference") (OtherBodyIndex :type Integer) (bFromSweep :type Boolean) (SweepResult :type "HitResult Structure (by ref)"))
  (bind _asbp_my_character (cast `/Game/SeongSik/Blueprints/Character/BP_MyCharacter` OtherActor))
  (`self.C2S_SetPlatformOwner` _asbp_my_character))

(event `self.ControlArea.OnComponentEndOverlap`
  (params (OverlappedComponent :type "PrimitiveComponent Object Reference") (OtherActor :type "Actor Object Reference") (OtherComp :type "PrimitiveComponent Object Reference") (OtherBodyIndex :type Integer))
  (bind _asbp_my_character (cast `/Game/SeongSik/Blueprints/Character/BP_MyCharacter` OtherActor)
    (:`then`
      (`self.C2S_SetPlatformOwner` _asbp_my_character))
    (:`CastFailed`
      (cast `/Game/SeongSik/Blueprints/Objects/BP_InteractableActor` OtherActor))))

(event `C2S_SetPlatformOwner`
  (params (InActor :type "/Game/SeongSik/Blueprints/Character/BP_MyCharacter Object Reference"))
  (`self.RequestProcessOwn` InActor))

(event `self.StaticMesh.OnComponentBeginOverlap`
  (params (OverlappedComponent :type "PrimitiveComponent Object Reference") (OtherActor :type "Actor Object Reference") (OtherComp :type "PrimitiveComponent Object Reference") (OtherBodyIndex :type Integer) (bFromSweep :type Boolean) (SweepResult :type "HitResult Structure (by ref)"))
  (bind _asbp_interactable_actor (cast `/Game/SeongSik/Blueprints/Objects/BP_InteractableActor` OtherActor))
  (`self.C2S_SetAttachActor` _asbp_interactable_actor))

(event `C2S_SetAttachActor`
  (params (InActor :type "/Game/SeongSik/Blueprints/Objects/BP_InteractableActor Object Reference"))
  (bind _asbp_my_gm (cast `/Game/SeongSik/Blueprints/BP_MyGM` (`GameplayStatics.GetGameMode`)))
  (`/Game/SeongSik/Blueprints/BP_MyGM.ProcessAttachActor` _asbp_my_gm self InActor))

(fn `RequestProcessOwn`
  (params (InCharacter :type "/Game/SeongSik/Blueprints/Character/BP_MyCharacter Object Reference"))
  (bind _asbp_my_gm (cast `/Game/SeongSik/Blueprints/BP_MyGM` (`GameplayStatics.GetGameMode`)))
  (`/Game/SeongSik/Blueprints/BP_MyGM.ProcessOwnPlatform` _asbp_my_gm self InCharacter))

(fn `UserConstructionScript`
  (`parent.UserConstructionScript`))